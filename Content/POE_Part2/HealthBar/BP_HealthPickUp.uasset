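; BP_HealthPickUp is a respawning health pickup collected on trigger overlap by the player or an AI.
; A Player-tagged BP_FPS_Character gets IncreaseHealth, while a BP_AI gets AdjustHealth with a negative amount of equal size.
; Both paths then hide the mesh and disable the trigger's overlaps, restoring them after a short delay.
; Any other untagged actor only triggers debug prints.
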(event OnComponentBeginOverlap(Trigger)
  (params (OverlappedComponent :type Primitive%20Component%20Object%20Reference) (OtherActor :type Actor%20Object%20Reference) (OtherComp :type Primitive%20Component%20Object%20Reference) (OtherBodyIndex :type Integer) (bFromSweep :type Boolean) (SweepResult :type Hit%20Result%20Structure%20%28by%20ref%29))
  (CallFunction|Collect OtherActor))

(event EventCollect
  (params (NewParam :type Actor%20Object%20Reference))
  (if (Actor|ActorHasTag NewParam "Player")
    (bind _asbp_fps_character (Utilities|Casting|CastToBP_FPS_Character NewParam))
    (Default|IncreaseHealth _asbp_fps_character 25.0)
    (Rendering|SetVisibility (Variables|Default|GetStaticMesh) false false :!label _label)
    (Variables|/Script/Engine.PrimitiveComponent|SetbGenerateOverlapEvents (Variables|Default|GetTrigger) false)
    (Utilities|FlowControl|Delay 5.0)
    (Rendering|SetVisibility (Variables|Default|GetStaticMesh) true false)
    (Variables|/Script/Engine.PrimitiveComponent|SetbGenerateOverlapEvents (Variables|Default|GetTrigger) true)
    (else
      (bind _asbp_ai (Utilities|Casting|CastToBP_AI NewParam)
        (:then
          (Default|AdjustHealth _asbp_ai -25.0)
          (goto _label))
        (:CastFailed
          (Development|PrintString "Fuckity")
          (Development|PrintString (Utilities|GetDisplayName NewParam)))))))

(fn ConstructionScript)