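; BP_AI is an enemy bot that shoots the player on sight and mirrors its health to the AI blackboard.
; Pawn sensing turns it toward the player, spawns a laser projectile, applies damage directly and flags the player as seen, throttled by a cooldown.
; Lethal damage asks GM_GameMode to respawn that bot class before destroying it.
; AdjustHealth also changes health but destroys without requesting a respawn.
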(event OnSeePawn(PawnSensing)
  (params (Pawn :type Pawn%20Object%20Reference))
  ;[0.15 0.15 0.15 0.5] Chase Player
  (bind _asbp_fps_character (Utilities|Casting|CastToBP_FPS_Character Pawn))
  (Transformation|SetActorRotation (Math|Rotator|FindRelativeLookatRotation (Math|Conversions|ToTransform(Vector) (Transformation|GetActorLocation)) (Transformation|GetActorLocation _asbp_fps_character)))
  (if (Variables|Default|GetCanAttack?)
    (Game|SpawnActorfromClass "/Game/POE_Part2/AI/Models/BP_LazerProjectile.BP_LazerProjectile_C" (Transformation|GetWorldTransform (Variables|Default|GetSpawnLocstion)) "Undefined" "MultiplyWithRoot" 0 0)
    (AI|Components|Blackboard|SetValueasBool (AI|GetBlackboard (AI|GetAIController self)) (Utilities|Name|MakeLiteralName "hasSeenPlayer") true)
    (Game|Damage|ApplyDamage _asbp_fps_character 12.0 0 0)
    (Variables|Default|SetCanAttack? false)
    (Utilities|FlowControl|Delay 1.0)
    (Variables|Default|SetCanAttack? true)))

(event EventBeginPlay
  (AI|Components|Blackboard|SetValueasFloat (AI|GetBlackboard 0) (Utilities|Name|MakeLiteralName "Health") 1e+02))

(event Game|Damage|EventAnyDamage
  (params (Damage :type Float%20%28single-precision%29) (DamageType :type Damage%20Type%20Object%20Reference) (InstigatedBy :type Controller%20Object%20Reference) (DamageCauser :type Actor%20Object%20Reference))
  ;[0.15 0.15 0.15 0.5] Damage Taken Stuff
  (bind _output_get (Variables|Default|SetEnemyHealth (- (Variables|Default|GetEnemyHealth) Damage)))
  (if (<= _output_get 0.0)
    (bind _asgm_game_mode (Utilities|Casting|CastToGM_GameMode (Game|GetGameMode)))
    (Default|RespawnSpecificBot _asgm_game_mode (Utilities|GetClass self))
    (Actor|DestroyActor)
    (else
      (AI|Components|Blackboard|SetValueasFloat (AI|GetBlackboard 0) (Utilities|Name|MakeLiteralName "Health") _output_get))))

(fn ConstructionScript)

(fn AdjustHealth
  (params (HealthDifference :type Float%20%28double-precision%29))
  (bind _output_get (Variables|Default|SetEnemyHealth (- (Variables|Default|GetEnemyHealth) HealthDifference)))
  (if (<= _output_get 0.0)
    (Actor|DestroyActor)
    (else
      (AI|Components|Blackboard|SetValueasFloat (AI|GetBlackboard 0) (Utilities|Name|MakeLiteralName "Health") _output_get))))