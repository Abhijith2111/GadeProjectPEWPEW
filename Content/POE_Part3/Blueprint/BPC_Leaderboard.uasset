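; Actor component, by its BPC prefix, that keeps a kill leaderboard for players.
; AddKill increments the player's count in the Leaderboard map, then rebuilds the TopPlayers array from its keys.
; A selection-sort-style nested loop aims to order TopPlayers by descending kills.
; It compares against the current element rather than the running maximum, swapping in the last higher scorer, so full ordering is not guaranteed.
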(event EventBeginPlay)

(event EventTick
  (params (DeltaSeconds :type Float%20%28single-precision%29)))

(fn AddKill
  (params (Player :type String))
  (bind _leaderboard (Variables|Default|GetLeaderboard))
  (bind _topplayers (Variables|Default|GetTopPlayers))
  (bind _leaderboard_2 (Variables|Default|GetLeaderboard))
  (bind (_value _returnvalue) (Utilities|Map|Find _leaderboard Player))
  (if _returnvalue
    (bind _result (Math|Integer|IncrementInt _value)
      (:%20%20
        (Utilities|Map|Add (Variables|Default|GetLeaderboard) Player _result)))
    (else
      (Utilities|Map|Add _leaderboard Player 1)))
  (Utilities|Array|Clear _topplayers)
  (bind _keypin (Utilities|Map|ForEachLoop(Map) _leaderboard)
    (:then
      (Utilities|Array|Add _topplayers _keypin))
    (:CompletedPin
      (for (_array_element _array_index) _topplayers
        (LocalVariables|SetMaxIndex _array_index)
        (for (_array_element_2 _array_index_2) _topplayers
          (if (> _array_index_2 _array_index)
            (if (.ReturnValue (Utilities|Map|Find _leaderboard_2 _array_element))
              (if (.ReturnValue (Utilities|Map|Find _leaderboard_2 _array_element_2))
                (if (> (.Value (Utilities|Map|Find _leaderboard_2 _array_element_2)) (.Value (Utilities|Map|Find _leaderboard_2 _array_element)))
                  (LocalVariables|SetMaxIndex _array_index_2))))))
        (Utilities|Array|Swap (Variables|Default|GetTopPlayers) _array_index (LocalVariables|GetMaxIndex))))))